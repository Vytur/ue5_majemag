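; BP_Door is an interactable, networked door that swings open and closed.
; Interact toggles IsOpen only on the authority, and the OnRep_isOpen notify turns that state into OpenDoor or CloseDoor.
; A single timeline plays forward to open and reverses to close, driving the door's relative yaw through its OpenClose track.
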(event Custom|ToggleDoor
  (Variables|Default|SetisOpen (not (Variables|Default|GetisOpen))))

(event Custom|CloseDoor
  (bind _openclose (Timeline|Timeline Reverse)
    (:Update
      (Transformation|SetRelativeRotation (Variables|Default|GetDoor) (Math|Rotator|MakeRotator 0.0 0.0 _openclose) false false))))

(event Custom|OpenDoor
  (bind _openclose (Timeline|Timeline Play)
    (:Update
      (Transformation|SetRelativeRotation (Variables|Default|GetDoor) (Math|Rotator|MakeRotator 0.0 0.0 _openclose) false false))))

(event EventInteract
  (Networking|SwitchHasAuthority
    (:Authority
      (CallFunction|ToggleDoor))))

(fn ConstructionScript
  (|CallParentFunction))

(fn OnRepIsOpen
  (if (Variables|Default|GetisOpen)
    (CallFunction|OpenDoor)
    (else
      (CallFunction|CloseDoor))))